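; BP_CheckPoint is a checkpoint actor that becomes the player's respawn location when touched.
; On overlap of its Checkpoint component, it sets the ThirdPersonCharacter's SpawnPoint to its own location, skipping if it already matches.
; A new activation also raises the ThirdPersonGameMode's SPtrigger flag and shows a particle effect, then clears both after a short delay.
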(event `self.checkpoint.OnComponentBeginOverlap`
  (params (OverlappedComponent :type "PrimitiveComponent Object Reference") (OtherActor :type "Actor Object Reference") (OtherComp :type "PrimitiveComponent Object Reference") (OtherBodyIndex :type Integer) (bFromSweep :type Boolean) (SweepResult :type "HitResult Structure (by ref)"))
  (bind _returnvalue (`self.K2_GetActorLocation`))
  (bind _asthird_person_character (cast `/Game/CustomContent/Blueprints/Player/ThirdPersonCharacter` OtherActor))
  (if (not (== _returnvalue (`/Game/CustomContent/Blueprints/Player/ThirdPersonCharacter.SpawnPoint` _asthird_person_character)))
    (set `/Game/CustomContent/Blueprints/Player/ThirdPersonCharacter.SpawnPoint` _returnvalue _asthird_person_character)
    (bind _asthird_person_game_mode (cast `/Game/CustomContent/Blueprints/ThirdPersonGameMode` (`GameplayStatics.GetGameMode`)))
    (set `/Game/CustomContent/Blueprints/ThirdPersonGameMode.SPtrigger` true _asthird_person_game_mode)
    (`SceneComponent.SetVisibility` (`self.ParticleSystem`) true false)
    (`KismetSystemLibrary.Delay` 2.0)
    (set `/Game/CustomContent/Blueprints/ThirdPersonGameMode.SPtrigger` false _asthird_person_game_mode)
    (`SceneComponent.SetVisibility` (`self.ParticleSystem`) false false)))

(fn `UserConstructionScript`)