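; BP_Returning_Platform is a moving platform that travels while the player character overlaps its Startpoint and returns when they leave.
; Overlap begin plays the Movement timeline and overlap end reverses it, both filtered to ThirdPersonCharacter.
; The timeline update lerps the Cube's relative location between PointA and PointB without sweeping.
; The construction script applies the Playrate variable to the timeline to set travel speed.
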(event `self.startpoint.OnComponentBeginOverlap`
  (params (OverlappedComponent :type "PrimitiveComponent Object Reference") (OtherActor :type "Actor Object Reference") (OtherComp :type "PrimitiveComponent Object Reference") (OtherBodyIndex :type Integer) (bFromSweep :type Boolean) (SweepResult :type "HitResult Structure (by ref)"))
  (cast `/Game/CustomContent/Blueprints/Player/ThirdPersonCharacter` OtherActor)
  (bind (_direction _newtrack_0) (`Timeline|Movement` :!label _label)
    (:`Update`
      (`SceneComponent.K2_SetRelativeLocation` (`self.Cube`) (`KismetMathLibrary.VLerp` (`self.PointA`) (`self.PointB`) _newtrack_0) false false))))

(event `self.startpoint.OnComponentEndOverlap`
  (params (OverlappedComponent :type "PrimitiveComponent Object Reference") (OtherActor :type "Actor Object Reference") (OtherComp :type "PrimitiveComponent Object Reference") (OtherBodyIndex :type Integer))
  (cast `/Game/CustomContent/Blueprints/Player/ThirdPersonCharacter` OtherActor)
  (goto _label :!via `Reverse`))

(fn `UserConstructionScript`
  (`parent.UserConstructionScript`)
  (`TimelineComponent.SetPlayRate` (`self.Movement`) (`self.playrate`)))