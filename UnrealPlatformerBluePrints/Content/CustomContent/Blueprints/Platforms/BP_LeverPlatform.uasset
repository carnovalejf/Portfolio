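; BP_LeverPlatform is a platform moved between two points by a lever, usable once the player has collected its activator.
; Touching the activator enables movement, brightens a light and destroys the pickup.
; The lever zone registers the lever on the character and shows a GameMode prompt.
; LeverTrigger checks both conditions, then plays or reverses a timeline lerping the cube's relative location, choosing direction by comparing world location to PointA.
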(event `self.ReceiveBeginPlay`
  (`parent.ReceiveBeginPlay`)
  (`self.EnableInput` (`GameplayStatics.GetPlayerController` 0)))

(event `self.activatorcollision.OnComponentBeginOverlap`
  (params (OverlappedComponent :type "PrimitiveComponent Object Reference") (OtherActor :type "Actor Object Reference") (OtherComp :type "PrimitiveComponent Object Reference") (OtherBodyIndex :type Integer) (bFromSweep :type Boolean) (SweepResult :type "HitResult Structure (by ref)"))
  (cast `/Game/CustomContent/Blueprints/Player/ThirdPersonCharacter` OtherActor)
  (set `self.canMove` true)
  (`LightComponent.SetIntensity` (`self.PointLight`) 3000.0)
  (`ActorComponent.K2_DestroyComponent` (`self.activatorcollision`))
  (`ActorComponent.K2_DestroyComponent` (`self.Activator`)))

(event `self.LeverZone.OnComponentBeginOverlap`
  (params (OverlappedComponent :type "PrimitiveComponent Object Reference") (OtherActor :type "Actor Object Reference") (OtherComp :type "PrimitiveComponent Object Reference") (OtherBodyIndex :type Integer) (bFromSweep :type Boolean) (SweepResult :type "HitResult Structure (by ref)"))
  (bind _asthird_person_character (cast `/Game/CustomContent/Blueprints/Player/ThirdPersonCharacter` OtherActor))
  (set `self.PlayerInRange` true)
  (set `/Game/CustomContent/Blueprints/Player/ThirdPersonCharacter.LeverRef` self _asthird_person_character)
  (bind _asthird_person_game_mode (cast `/Game/CustomContent/Blueprints/ThirdPersonGameMode` (`GameplayStatics.GetGameMode`)))
  (set `/Game/CustomContent/Blueprints/ThirdPersonGameMode.Instruction` "Press E To Activate When Bright" _asthird_person_game_mode))

(event `self.LeverZone.OnComponentEndOverlap`
  (params (OverlappedComponent :type "PrimitiveComponent Object Reference") (OtherActor :type "Actor Object Reference") (OtherComp :type "PrimitiveComponent Object Reference") (OtherBodyIndex :type Integer))
  (cast `/Game/CustomContent/Blueprints/Player/ThirdPersonCharacter` OtherActor)
  (set `self.PlayerInRange` false)
  (bind _asthird_person_game_mode (cast `/Game/CustomContent/Blueprints/ThirdPersonGameMode` (`GameplayStatics.GetGameMode`)))
  (set `/Game/CustomContent/Blueprints/ThirdPersonGameMode.Instruction` "" _asthird_person_game_mode))

(event `LeverTrigger`
  (bind _move (`self.Activate`))
  (if _move
    (`/Game/CustomContent/Blueprints/Player/ThirdPersonCharacter.UsingLever` (stale `self.LeverZone.OnComponentBeginOverlap` _asthird_person_character))
    (if (== (`SceneComponent.K2_GetComponentLocation` (`self.Cube`)) (`self.PointA`))
      (bind (_direction _newtrack_0) (`Timeline|Timeline_0` :!label _label)
        (:`Update`
          (`SceneComponent.K2_SetRelativeLocation` (`self.Cube`) (`KismetMathLibrary.VLerp` (`self.PointA`) (`self.PointB`) _newtrack_0) false false)))
      (else
        (goto _label :!via `Reverse`)))))

(fn `Activate`
  (returns (Move :type Boolean))
  (return (and (`self.canMove`) (`self.PlayerInRange`))))

(fn `UserConstructionScript`
  (`parent.UserConstructionScript`))