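; BP_AutoPlatform is a platform whose Cube moves back and forth automatically between PointA and PointB, pausing two seconds at each end.
; Each Tick compares the Cube's world location to both points and, after the delay, plays or reverses the Movement timeline.
; The timeline lerps the Cube's relative location between the points without sweeping, although the endpoint checks use world location.
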(event `self.ReceiveTick`
  (params (DeltaSeconds :type "Float (single-precision)"))
  (bind _returnvalue (`SceneComponent.K2_GetComponentLocation` (`self.Cube`)))
  (if (== _returnvalue (`self.PointA`))
    (`KismetSystemLibrary.Delay` 2.0)
    (bind (_direction _newtrack_0) (`Timeline|Movement` :!label _label)
      (:`Update`
        (`SceneComponent.K2_SetRelativeLocation` (`self.Cube`) (`KismetMathLibrary.VLerp` (`self.PointA`) (`self.PointB`) _newtrack_0) false false)))
    (elif (== _returnvalue (`self.PointB`))
      (`KismetSystemLibrary.Delay` 2.0)
      (goto _label :!via `Reverse`))))

(fn `UserConstructionScript`
  (`parent.UserConstructionScript`))